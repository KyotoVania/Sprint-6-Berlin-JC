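; BP_Item_Crystals is a crystal item whose look is set by its emotion type: Anger, Sadness, Hope, Joy, Fear or Remission.
; On BeginPlay, the type selects material, particle effect and light color, which are applied to the shared mesh, particle component and point light.
; A timeline animates the mesh's relative height.
; An attached attenuated sound is wired up, but every type leaves it empty.
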(event `self.ReceiveBeginPlay`
  (bind _sm_shape (`self.SM_Shape`))
  (switch `/Game/00-Blueprints/Enumerations/E_CrystalsType` (`self.CrystalType`)
    (:`NewEnumerator0`
      (set `self.CrystalSFX` null)
      (set `self.CrystalMesh` "/Game/Crystals/Mesh/SM_Crystal_3.SM_Crystal_3")
      (set `self.CrystalMaterial` "/Game/Crystals/Material/M_Crystal_Inst3.M_Crystal_Inst3")
      (set `self.CrystalVFX` "/Game/Crystals/Particles/P_Crystal_3.P_Crystal_3")
      (set `self.LightColor` (struct :`R` 1.0 :`G` 0.145098 :`B` 0.145098 :`A` 1.0)))
    (:`NewEnumerator1`
      (set `self.CrystalSFX` null)
      (set `self.CrystalMesh` "/Game/Crystals/Mesh/SM_Crystal_3.SM_Crystal_3")
      (set `self.CrystalMaterial` "/Game/Crystals/Material/M_Crystal_Inst4.M_Crystal_Inst4")
      (set `self.CrystalVFX` "/Game/Crystals/Particles/P_Crystal_5.P_Crystal_5")
      (set `self.LightColor` (struct :`R` 0.105882 :`G` 0.454902 :`B` 1.0 :`A` 1.0)))
    (:`NewEnumerator2`
      (set `self.CrystalSFX` null)
      (set `self.CrystalMesh` "/Game/Crystals/Mesh/SM_Crystal_3.SM_Crystal_3")
      (set `self.CrystalMaterial` "/Game/Crystals/Material/M_Crystal_Inst6.M_Crystal_Inst6")
      (set `self.CrystalVFX` "/Game/Crystals/Particles/P_Crystal_7.P_Crystal_7")
      (set `self.LightColor` (struct :`R` 0.176471 :`G` 1.0 :`B` 0.223529 :`A` 1.0)))
    (:`NewEnumerator3`
      (set `self.CrystalSFX` null)
      (set `self.CrystalMesh` "/Game/Crystals/Mesh/SM_Crystal_3.SM_Crystal_3")
      (set `self.CrystalMaterial` "/Game/Crystals/Material/M_Crystal_Inst9_2.M_Crystal_Inst9_2")
      (set `self.CrystalVFX` "/Game/Crystals/Particles/P_Crystal_9.P_Crystal_9")
      (set `self.LightColor` (struct :`R` 1.0 :`G` 0.905882 :`B` 0.235294 :`A` 1.0)))
    (:`NewEnumerator4`
      (set `self.CrystalSFX` null)
      (set `self.CrystalMesh` "/Game/Crystals/Mesh/SM_Crystal_3.SM_Crystal_3")
      (set `self.CrystalMaterial` "/Game/Crystals/Material/M_Crystal_Inst1_2.M_Crystal_Inst1_2")
      (set `self.CrystalVFX` "/Game/Crystals/Particles/P_Crystal_1.P_Crystal_1")
      (set `self.LightColor` (struct :`R` 1.0 :`G` 0.266667 :`B` 0.980392 :`A` 1.0)))
    (:`NewEnumerator5`
      (set `self.CrystalSFX` null)
      (set `self.CrystalMesh` "/Game/Crystals/Mesh/SM_Crystal_3.SM_Crystal_3")
      (set `self.CrystalMaterial` "/Game/Crystals/Material/M_Crystal_Inst10.M_Crystal_Inst10")
      (set `self.CrystalVFX` "/Game/Crystals/Particles/P_Crystal_10.P_Crystal_10")
      (set `self.LightColor` (struct :`R` 1.0 :`G` 0.356863 :`B` 0.121569 :`A` 1.0))))
  (`GameplayStatics.SpawnSoundAttached` (`self.CrystalSFX`) (`self.SM_Shape`) "None" (0.0 0.0 0.0) (struct) "KeepRelativeOffset" false 1.0 1.0 0.0 "/Game/02-Musics_SFX/SA_Crystals.SA_Crystals" null)
  (`StaticMeshComponent.SetStaticMesh` _sm_shape (`self.CrystalMesh`))
  (`PrimitiveComponent.SetMaterial` _sm_shape 0 (`self.CrystalMaterial`))
  (`ParticleSystemComponent.SetTemplate` (`self.P_Crystal_1`) (`self.CrystalVFX`))
  (`LightComponent.SetLightColor` (`self.PointLight`) (`self.LightColor`) true)
  (bind (_direction _z) (`Timeline|Timeline`)
    (:`Update`
      (`SceneComponent.K2_SetRelativeLocation` (`self.SM_Shape`) (`KismetMathLibrary.MakeVector` 0.0 0.0 _z) false false))))

(fn `UserConstructionScript`
  (`parent.UserConstructionScript`))